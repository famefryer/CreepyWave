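; MyPawn is a pawn pushed forward or backward by physics forces on its static mesh.
; W and S key presses call MoveForward with opposite directions, so force is applied once per press rather than every tick.
; MoveForward applies force along the mesh's forward vector, scaled by its mass, a gravity-sized constant and a speed multiplier set at BeginPlay.
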(event `self.ReceiveBeginPlay`
  (set `self.multiplySpeed` 10.0))

(event `Key|W`
  (params (Key :type "Key Structure"))
  (:`Pressed`
    (`self.MoveForward` 1)))

(event `Key|S`
  (params (Key :type "Key Structure"))
  (:`Pressed`
    (`self.MoveForward` -1)))

(fn `MoveForward`
  (params (Direction :type Integer))
  (bind _staticmesh (`self.StaticMesh`))
  (`PrimitiveComponent.AddForce` _staticmesh (* (`SceneComponent.GetForwardVector` _staticmesh) (* (* (* Direction (`PrimitiveComponent.GetMass` _staticmesh)) 980.0) (`self.multiplySpeed`))) "None" false))

(fn `UserConstructionScript`)