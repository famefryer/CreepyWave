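; Player controller that runs a wave-based snowman shooter: start menu, Tab pause, score, player health and game over.
; StartGame clears monsters, counts down, then spawns delayed batches of small snowmen at random SpawnPlace actors and scaled big snowmen within those actors' XY bounds.
; Hit and kill functions adjust score or health, returning to the menu at zero health.
; StartNextWave raises monster counts and big-snowman size before restarting the countdown.
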(event `Key|Tab`
  (params (Key :type "Key Structure"))
  (:`Pressed`
    (`GameplayStatics.SetGamePaused` true)
    (set `self.bShowMouseCursor` true)))

(event `self.ReceiveBeginPlay`
  (`self.MainMenu`)
  (bind _outactors (`GameplayStatics.GetAllActorsOfClass` "/Game/StarterContent/Blueprints/SpawnPlace.SpawnPlace_C"))
  (set `self.Spawnplaces` _outactors)
  (`self.CalculateScopeOfSpawnPlace`))

(event `self.ReceiveTick`
  (params (DeltaSeconds :type "Float (single-precision)")))

(event `Spawn Monster`
  (bind _bigmonstersize (`self.BigMonsterSize`))
  ;[1 1 1] Small Monster Spawn
  (`/Game/Blueprints/CustomLoop.ForLoopWithDelay` 0 (* (`self.SnowmanNumber`) (`self.WaveNumber`)) 0.3
    (:`LoopBody`
      (bind _transform (`self.RandomSpawnPlace` 1.0))
      (`|SpawnActorFromClass` "/Game/Blueprints/CreepySnowman.CreepySnowman_C" _transform "Undefined" "OverrideRootScale" null null))
    (:`Completed`
      ;[1 1 1] Big Monster Spawn
      (`/Game/Blueprints/CustomLoop.ForLoopWithDelay` 1 (* (`self.WaveNumber`) (`self.BigSnowmanNumber`)) 0.5
        (:`LoopBody`
          (`|SpawnActorFromClass` "/Game/Blueprints/BigSnowman.BigSnowman_C" (`KismetMathLibrary.MakeTransform` (`KismetMathLibrary.MakeVector` (`KismetMathLibrary.RandomFloatInRange` (`self.MonsSpawnMinX`) (`self.MonsSpawnMaxX`)) (`KismetMathLibrary.RandomFloatInRange` (`self.MonsSpawnMinY`) (`self.MonsSpawnMaxY`)) (- (* 100.0 _bigmonstersize) 50.0)) (struct) (`KismetMathLibrary.MakeVector` _bigmonstersize _bigmonstersize _bigmonstersize)) "Undefined" "OverrideRootScale" null null))))))

(event `StartGame`
  (`self.ClearAllMonster`)
  (set `PlayerController.bShowMouseCursor` false (`GameplayStatics.GetPlayerController` 0))
  (if (!= (`self.WaveNumber`) 1)
    (`/Game/Blueprints/CustomLoop.ForLoopWithDelay` 0 (`self.WaitTimeBetweenWave`) 1.0
      (:`LoopBody`
        (set `self.WaveCountDown` (- (`self.WaveCountDown`) 1) :!label _label))
      (:`Completed`
        (set `self.isGameStart` true :!label _label_2)
        (`self.Spawn Monster`)
        (`GameplayStatics.SetGamePaused` false)))
    (else
      (`/Game/Blueprints/CustomLoop.ForLoopWithDelay` 0 3 1.0
        (:`LoopBody`
          (goto _label))
        (:`Completed`
          (goto _label_2))))))

(fn `BigSnowmanHitPlayer`
  (bind _output_get (set `self.PlayerHealth` (- (`self.PlayerHealth`) 0.2)))
  (if (<= _output_get 0.0)
    (`self.GameOver`)))

(fn `CalculateScopeOfSpawnPlace`
  (for _array_element (`self.Spawnplaces`)
    (bind (_returnvalue_x _returnvalue_y) (`KismetMathLibrary.BreakVector` (`SceneComponent.K2_GetComponentLocation` (`/Game/StarterContent/Blueprints/SpawnPlace.StaticMesh` _array_element))))
    (if (< _returnvalue_x (`self.MonsSpawnMinX`))
      (set `self.MonsSpawnMinX` _returnvalue_x))
    (if (> _returnvalue_x (`self.MonsSpawnMaxX`))
      (set `self.MonsSpawnMaxX` _returnvalue_x))
    (if (< _returnvalue_y (`self.MonsSpawnMinY`))
      (set `self.MonsSpawnMinY` _returnvalue_y))
    (if (> _returnvalue_y (`self.MonsSpawnMaxY`))
      (set `self.MonsSpawnMaxY` _returnvalue_y))))

(fn `ClearAllMonster`
  (bind _outactors (`GameplayStatics.GetAllActorsOfClass` "/Game/Blueprints/CreepySnowman.CreepySnowman_C"))
  (for _array_element _outactors
    (`self.K2_DestroyActor` _array_element))
  (bind _outactors_2 (`GameplayStatics.GetAllActorsOfClass` "/Game/Blueprints/BigSnowman.BigSnowman_C"))
  (for _array_element_2 _outactors_2
    (`self.K2_DestroyActor` _array_element_2)))

(fn `GameOver`
  (`WidgetLayoutLibrary.RemoveAllWidgets`)
  (`self.ClearAllMonster`)
  (`self.MainMenu`))

(fn `MainMenu`
  (bind _returnvalue (`GameplayStatics.GetPlayerController` 0))
  (set `PlayerController.bShowMouseCursor` true _returnvalue)
  (bind _returnvalue_2 (`|CreateWidget` "/Game/Blueprints/Widget/StartWidget.StartWidget_C" _returnvalue))
  (`UserWidget.AddToViewport` _returnvalue_2 0)
  (`GameplayStatics.SetGamePaused` true))

(fn `PlayerHitBigSnowman`
  (set `self.Score` (+ (`self.Score`) 50)))

(fn `PlayerHitSnowman`
  (set `self.Score` (+ (`self.Score`) 100)))

(fn `PlayerKillBigSnowman`
  (set `self.Score` (+ (`self.Score`) 3000)))

(fn `PlayerKillSnowman`
  (set `self.Score` (+ (`self.Score`) 300)))

(fn `RandomSpawnPlace`
  (params (MonsterSize :type "Float (double-precision)"))
  (returns (Transform :type "Transform Structure"))
  (bind _returnvalue (`KismetMathLibrary.RandomFloatInRange` 0.0 20.0))
  (bind _spawnplaces (`self.Spawnplaces`))
  (bind _rootcomponent (`Actor.RootComponent` (`|GetArrayItem` _spawnplaces (`KismetMathLibrary.RandomInteger` (- (`KismetArrayLibrary.Array_Length` _spawnplaces) 1)))))
  (bind (_returnvalue_x _returnvalue_y) (`KismetMathLibrary.BreakVector` (`SceneComponent.K2_GetComponentLocation` _rootcomponent)))
  (return (`KismetMathLibrary.MakeTransform` (`KismetMathLibrary.MakeVector` (- _returnvalue_x _returnvalue) (- _returnvalue_y _returnvalue) 160.0) (`SceneComponent.K2_GetComponentRotation` _rootcomponent) (`KismetMathLibrary.MakeVector` MonsterSize MonsterSize MonsterSize))))

(fn `SnowmanHitPlayer`
  (bind _output_get (set `self.PlayerHealth` (- (`self.PlayerHealth`) 0.01)))
  (if (<= _output_get 0.0)
    (`self.GameOver`)))

(fn `StartNextWave`
  (set `self.WaveCountDown` (+ (`self.WaitTimeBetweenWave`) 1))
  (set `self.WaveNumber` (+ (`self.WaveNumber`) 1))
  (set `self.SnowmanNumber` (+ (`self.SnowmanNumber`) 5))
  (set `self.BigSnowmanNumber` (+ (`self.BigSnowmanNumber`) 1))
  (set `self.BigMonsterSize` (+ (`self.BigMonsterSize`) 0.5))
  (`self.StartGame`))

(fn `UserConstructionScript`)