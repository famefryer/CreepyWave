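; MyChar is the player character for a snowman-fighting shooter, handling movement, look, jumping and two weapons.
; Left and right click spawn bullet or bazooka projectiles at BulletSpawnLoc, consuming ammo only once the game has started.
; C sets OpenShop when the game has not started and the cached MyPlayerController allows buying.
; Capsule hits from a CreepySnowman are reported through that snowman's PlayerController reference.
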(event `self.ReceiveBeginPlay`
  (bind _asmy_player_controller (cast `/Game/Blueprints/MyPlayerController` (`GameplayStatics.GetPlayerController` 0)))
  (set `self.playercontroller` _asmy_player_controller))

(event `InputAxis|RotateRight`
  (params (AxisValue :type "Float (single-precision)"))
  (`self.AddControllerYawInput` AxisValue))

(event `InputAxis|MoveForward`
  (params (AxisValue :type "Float (single-precision)"))
  (`self.AddMovementInput` (`KismetMathLibrary.GetForwardVector` (`self.GetControlRotation`)) AxisValue))

(event `InputAxis|RotateUp`
  (params (AxisValue :type "Float (single-precision)"))
  (`self.AddControllerPitchInput` AxisValue))

(event `InputAxis|MoveRight`
  (params (AxisValue :type "Float (single-precision)"))
  (`self.AddMovementInput` (`KismetMathLibrary.GetRightVector` (`self.GetControlRotation`)) AxisValue))

(event `Key|SpaceBar`
  (params (Key :type "Key Structure"))
  (:`Pressed`
    (`self.Jump`)))

(event `Key|C`
  (params (Key :type "Key Structure"))
  (bind _playercontroller (`self.playercontroller`))
  ;[1 1 1] Press C to Open Shop
  (:`Pressed`
    (if (`/Game/Blueprints/MyPlayerController.isGameStart` _playercontroller)
      _
      (elif (`/Game/Blueprints/MyPlayerController.canBuyFromShop` _playercontroller)
        (set `self.openShop` true)))))

(event `self.CapsuleComponent.OnComponentHit`
  (params (HitComponent :type "PrimitiveComponent Object Reference") (OtherActor :type "Actor Object Reference") (OtherComp :type "PrimitiveComponent Object Reference") (NormalImpulse :type "Vector Structure") (Hit :type "HitResult Structure (by ref)"))
  (bind _ascreepy_snowman (cast `/Game/Blueprints/CreepySnowman` OtherActor))
  (`/Game/Blueprints/MyPlayerController.SnowmanHitPlayer` (`/Game/Blueprints/CreepySnowman.playerController` _ascreepy_snowman)))

(event `Key|LeftMouseButton`
  (params (Key :type "Key Structure"))
  ;[1 1 1] Left Click to Shoot
  (:`Pressed`
    (if (not (<= (`self.Ammos`) 0))
      (bind _returnvalue (`|SpawnActorFromClass` "/Game/Blueprints/Bullet.Bullet_C" (`SceneComponent.K2_GetComponentToWorld` (`self.BulletSpawnLoc`)) "Undefined" "OverrideRootScale" null null))
      (`GameplayStatics.PlaySound2D` "/Game/ImportedAsset/Sounds/Gun+Silencer.Gun+Silencer" 0.18 1.0 0.0 null null)
      (`SceneComponent.SetWorldScale3D` (`/Game/Blueprints/Bullet.StaticMesh` _returnvalue) (0.5 0.5 0.5))
      (if (`/Game/Blueprints/MyPlayerController.isGameStart` (`self.playercontroller`))
        (set `self.Ammos` (- (`self.Ammos`) 1))))))

(event `Key|RightMouseButton`
  (params (Key :type "Key Structure"))
  ;[1 1 1] Right Click to use Bazooka
  (:`Pressed`
    (if (not (<= (`self.BazookaAmmos`) 0))
      (bind _returnvalue (`|SpawnActorFromClass` "/Game/Blueprints/BazookaBullet.BazookaBullet_C" (`SceneComponent.K2_GetComponentToWorld` (`self.BulletSpawnLoc`)) "Undefined" "OverrideRootScale" null null))
      (`GameplayStatics.PlaySound2D` "/Game/ImportedAsset/Sounds/Missile+2.Missile+2" 0.7 1.0 0.0 null null)
      (`SceneComponent.SetWorldScale3D` (`Actor.RootComponent` _returnvalue) (1.1 1.1 1.1))
      (if (`/Game/Blueprints/MyPlayerController.isGameStart` (`self.playercontroller`))
        (set `self.BazookaAmmos` (- (`self.BazookaAmmos`) 1))))))

(fn `UserConstructionScript`)