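; BigSnowman is an enemy actor that turns to face the player and fires enlarged MagicBullets at random intervals.
; Tick drives the smoothed rotation, with a random Delay pacing each spawn from BulletSpawnLoc.
; HittedByBullet counts hits on four body parts, recoloring each yellow, then red at thresholds.
; When all four reach the red threshold, it notifies MyPlayerController of the kill, spawns an explosion and destroys itself.
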(event `self.ReceiveBeginPlay`
  (bind _asmy_player_controller (cast `/Game/Blueprints/MyPlayerController` (`GameplayStatics.GetPlayerController` 0)))
  (set `self.PlayerController` _asmy_player_controller))

(event `self.ReceiveTick`
  (params (DeltaSeconds :type "Float (single-precision)"))
  (`self.FindPlayer` DeltaSeconds)
  (`KismetSystemLibrary.Delay` (`KismetMathLibrary.RandomFloatInRange` 1.0 5.0))
  (bind _returnvalue (`|SpawnActorFromClass` "/Game/Blueprints/MagicBullet.MagicBullet_C" (`KismetMathLibrary.MakeTransform` (`SceneComponent.K2_GetComponentLocation` (`self.BulletSpawnLoc`)) (`SceneComponent.K2_GetComponentRotation` (`self.Bottom`))) "Undefined" "OverrideRootScale" null null))
  (`SceneComponent.SetWorldScale3D` (`/Game/Blueprints/MagicBullet.StaticMesh` _returnvalue) (1.2 1.2 1.2)))

(fn `FindPlayer`
  (params (DeltaTime :type "Float (double-precision)"))
  (`self.K2_SetActorRotation` (`KismetMathLibrary.RInterpTo` (`self.K2_GetActorRotation`) (`KismetMathLibrary.FindLookAtRotation` (`self.K2_GetActorLocation`) (`self.K2_GetActorLocation` (`GameplayStatics.GetPlayerCharacter` 0))) DeltaTime 10.0)))

(fn `HittedByBullet`
  (params (PartThatHitted :type "StaticMeshComponent Object Reference"))
  (bind _partthathitted (`self.PartThatHitted`))
  (bind _partthathitted_2 (`self.PartThatHitted`))
  (bind _hitcountbottom (`self.HitCountBottom`))
  (bind _hitcountlowbody (`self.HitCountLowBody`))
  (bind _hitcountupbody (`self.HitCountUpBody`))
  (bind _hitcounthead (`self.HitCountHead`))
  (bind _bottom (`self.Bottom`))
  (bind _partthathitted_3 (`self.PartThatHitted`))
  (bind _output_get (set `self.PartThatHitted` PartThatHitted))
  ;[1 1 1] Check which part and set to hitted count
  (if (== _output_get (`self.Bottom`))
    (set `self.CountOfHittedPart` _hitcountbottom)
    (set `self.HitCountBottom` (+ _hitcountbottom 1))
    (switch `int` (`self.CountOfHittedPart`) :!label _label
      (:`5`
        ;[1 1 1] Change Color of hitted part
        (`PrimitiveComponent.SetMaterial` _partthathitted 0 "/Game/StarterContent/Yellow_Mat.Yellow_Mat")
        (`PrimitiveComponent.SetMaterial` _partthathitted_2 0 "/Game/StarterContent/Yellow_Mat.Yellow_Mat")
        (`PrimitiveComponent.SetMaterial` _partthathitted_3 0 "/Game/StarterContent/Yellow_Mat.Yellow_Mat"))
      (:`10`
        (`PrimitiveComponent.SetMaterial` _partthathitted 0 "/Game/StarterContent/Red_Mat.Red_Mat")
        (`PrimitiveComponent.SetMaterial` _partthathitted_2 0 "/Game/StarterContent/Red_Mat.Red_Mat")
        (`PrimitiveComponent.SetMaterial` _partthathitted_3 0 "/Game/StarterContent/Red_Mat.Red_Mat")
        ;[1 1 1] Check is every part turn to red
        (if (>= (`self.HitCountLowBody`) 10)
          (if (>= (`self.HitCountUpBody`) 10)
            (if (>= (`self.HitCountHead`) 10)
              (if (>= (`self.HitCountBottom`) 10)
                (`/Game/Blueprints/MyPlayerController.PlayerKillBigSnowman` (`self.PlayerController`))
                ;[1 1 1] Bomb and Destroy
                (`GameplayStatics.SpawnEmitterAtLocation` "/Game/StarterContent/Particles/P_Explosion.P_Explosion" (`SceneComponent.K2_GetComponentLocation` _bottom) (`SceneComponent.K2_GetComponentRotation` _bottom) (50.0 50.0 50.0))
                (`self.K2_DestroyActor`)))))))
    (elif (== _output_get (`self.LowBody`))
      (set `self.CountOfHittedPart` _hitcountlowbody)
      (set `self.HitCountLowBody` (+ _hitcountlowbody 1))
      (goto _label)
      (elif (== _output_get (`self.UpBody`))
        (set `self.CountOfHittedPart` _hitcountupbody)
        (set `self.HitCountUpBody` (+ _hitcountupbody 1))
        (goto _label)
        (elif (== _output_get (`self.Head`))
          (set `self.CountOfHittedPart` _hitcounthead)
          (set `self.HitCountHead` (+ _hitcounthead 1))
          (goto _label))))))

(fn `UserConstructionScript`)