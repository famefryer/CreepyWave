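; Enemy snowman that hops around facing the player until shot down.
; Tick smoothly rotates it toward the player, and any blocking non-bullet hit on its Bottom component applies a randomized, mass-scaled upward force.
; HittedByBullet, not called within this Blueprint, turns it yellow, then red, then explodes it on the third hit, notifying MyPlayerController of the kill before destroying it.
; Bazooka hits add two to the count first, killing it immediately.
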(event `self.ReceiveBeginPlay`
  (bind _asmy_player_controller (cast `/Game/Blueprints/MyPlayerController` (`GameplayStatics.GetPlayerController` 0)))
  (set `self.playerController` _asmy_player_controller))

(event `self.ReceiveTick`
  (params (DeltaSeconds :type "Float (single-precision)"))
  (`self.FindPlayer` DeltaSeconds))

(event `self.Bottom.OnComponentHit`
  (params (HitComponent :type "PrimitiveComponent Object Reference") (OtherActor :type "Actor Object Reference") (OtherComp :type "PrimitiveComponent Object Reference") (NormalImpulse :type "Vector Structure") (Hit :type "HitResult Structure (by ref)"))
  (bind (_bblockinghit _binitialoverlap _time _distance _location _impactpoint _normal _impactnormal _physmat _hitactor) (`GameplayStatics.BreakHitResult` Hit))
  (bind _bottom (`self.Bottom`))
  (if _bblockinghit
    (cast `/Game/Blueprints/Bullet` _hitactor
      (:`CastFailed`
        (`PrimitiveComponent.AddForce` _bottom (`KismetMathLibrary.MakeVector` 0.0 0.0 (* (* (`PrimitiveComponent.GetMass` _bottom) 980.0) (+ (`self.jumpForce`) (`KismetMathLibrary.RandomFloatInRange` 0.0 20.0)))) "None" false)))))

(fn `FindPlayer`
  (params (Delta :type "Float (double-precision)"))
  (`self.K2_SetActorRotation` (`KismetMathLibrary.RInterpTo` (`self.K2_GetActorRotation`) (`KismetMathLibrary.FindLookAtRotation` (`self.K2_GetActorLocation`) (`self.K2_GetActorLocation` (`GameplayStatics.GetPlayerCharacter` 0))) Delta 10.0)))

(fn `hittedByBullet`
  (params (isBazooka :type Boolean))
  (bind _body (`self.Body`))
  (if isBazooka
    (set `self.hitCount` (+ (`self.hitCount`) 2)))
  (switch `int` (`self.hitCount`)
    (:`Default`
      (`GameplayStatics.SpawnEmitterAtLocation` "/Game/StarterContent/Particles/P_Explosion.P_Explosion" (`SceneComponent.K2_GetComponentLocation` _body) (`SceneComponent.K2_GetComponentRotation` _body) :!label _label)
      (`/Game/Blueprints/MyPlayerController.PlayerKillSnowman` (`self.playerController`))
      (`self.K2_DestroyActor`))
    (:`0`
      (`PrimitiveComponent.SetMaterial` (`self.Body`) 0 "/Game/StarterContent/Yellow_Mat.Yellow_Mat")
      (`PrimitiveComponent.SetMaterial` (`self.Bottom`) 0 "/Game/StarterContent/Yellow_Mat.Yellow_Mat")
      (`PrimitiveComponent.SetMaterial` (`self.Head`) 0 "/Game/StarterContent/Yellow_Mat.Yellow_Mat")
      (set `self.hitCount` (+ (`self.hitCount`) 1) :!label _label_2))
    (:`1`
      (`PrimitiveComponent.SetMaterial` (`self.Body`) 0 "/Game/StarterContent/Red_Mat.Red_Mat")
      (`PrimitiveComponent.SetMaterial` (`self.Bottom`) 0 "/Game/StarterContent/Red_Mat.Red_Mat")
      (`PrimitiveComponent.SetMaterial` (`self.Head`) 0 "/Game/StarterContent/Red_Mat.Red_Mat")
      (goto _label_2))
    (:`2`
      (goto _label))))

(fn `UserConstructionScript`)