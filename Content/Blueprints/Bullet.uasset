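; Bullet projectile actor that damages snowman enemies and fires a radial force impulse on any blocking hit.
; It caches MyPlayerController on BeginPlay to report snowman hits, passing false for the bazooka flag.
; A CreepySnowman hit destroys the bullet immediately, while other non-snowman hits destroy it after a short delay.
; BigSnowman hits forward the struck mesh component and leave the bullet alive; a spark emitter is unwired.
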(event `self.ReceiveBeginPlay`
  (bind _asmy_player_controller (cast `/Game/Blueprints/MyPlayerController` (`GameplayStatics.GetPlayerController` 0)))
  (set `self.playerController` _asmy_player_controller))

(event `self.StaticMesh.OnComponentHit`
  (params (HitComponent :type "PrimitiveComponent Object Reference") (OtherActor :type "Actor Object Reference") (OtherComp :type "PrimitiveComponent Object Reference") (NormalImpulse :type "Vector Structure") (Hit :type "HitResult Structure (by ref)"))
  (bind _playercontroller (`self.PlayerController`))
  (if Hit_bBlockingHit
    (`RadialForceComponent.FireImpulse` (`self.RadialForce`))
    (bind _ascreepy_snowman (cast `/Game/Blueprints/CreepySnowman` OtherActor)
      (:`then`
        (`/Game/Blueprints/CreepySnowman.hittedByBullet` _ascreepy_snowman false)
        (`/Game/Blueprints/MyPlayerController.PlayerHitSnowman` _playercontroller false)
        (`self.K2_DestroyActor` :!label _label))
      (:`CastFailed`
        (bind _asbig_snowman (cast `/Game/Blueprints/BigSnowman` OtherActor)
          (:`then`
            (bind _asstatic_mesh_component (cast `StaticMeshComponent` OtherComp))
            (`/Game/Blueprints/MyPlayerController.PlayerHitBigSnowman` _playercontroller false)
            (`/Game/Blueprints/BigSnowman.HittedByBullet` _asbig_snowman _asstatic_mesh_component false))
          (:`CastFailed`
            (`KismetSystemLibrary.Delay` 1.0)
            (goto _label)))))))

(fn `UserConstructionScript`)